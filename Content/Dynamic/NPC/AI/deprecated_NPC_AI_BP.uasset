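; Deprecated AI controller for guard NPCs that starts the patrol blackboard and guard behavior tree on BeginPlay.
; AI perception updates set sensed actors without the Guard tag as the blackboard Enemy and clear that key when such an actor is lost.
; A debug helper that prints the guard, sense class and perceived object exists but is never called at runtime.
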(event `self.AIPerception.OnTargetPerceptionUpdated`
  (params (Actor :type "Actor Object Reference") (Stimulus :type "AIStimulus Structure"))
  (bind _returnvalue (`KismetStringLibrary.Conv_StringToName` "Enemy"))
  (bind _patrolblackboard (`self.PatrolBlackboard`))
  (if (`self.ActorHasTag` Actor "Guard")
    _
    (elif (`.bSuccessfullySensed` (break `AIStimulus` Stimulus))
      (`BlackboardComponent.SetValueAsObject` _patrolblackboard _returnvalue Actor)
      (else
        (`BlackboardComponent.ClearValue` _patrolblackboard _returnvalue)))))

(event `self.ReceiveBeginPlay`
  (bind _blackboardcomponent (`self.UseBlackboard` "/Game/Dynamic/NPC/AI/PatrolData.PatrolData"))
  (set `self.PatrolBlackboard` _blackboardcomponent)
  (`self.RunBehaviorTree` "/Game/Dynamic/NPC/AI/GuardBehavior.GuardBehavior"))

(fn `Display Perception Event`
  (params (Stimulus :type "AIStimulus Structure (by ref)") (Object :type "Object Object Reference"))
  (bind _returnvalue (`AIPerceptionSystem.GetSenseClassForStimulus` Stimulus))
  (`KismetSystemLibrary.PrintString` (`KismetStringLibrary.Concat_StrStr` "Guard " (`KismetSystemLibrary.GetDisplayName` (`self.K2_GetPawn`)) " <" (`KismetSystemLibrary.GetClassDisplayName` _returnvalue) "> " (`KismetSystemLibrary.GetDisplayName` Object))))

(fn `UserConstructionScript`)